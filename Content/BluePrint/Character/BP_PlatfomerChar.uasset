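; BP_PlatfomerChar is a sprite-based platformer character Blueprint that handles the character's defeat.
; Defeat runs once, disabling capsule collision and the movement plane constraint, then launching the character up and along the world right axis by tunable amounts.
; It also jumps the animation state machine to a defeated node and raises the sprite's translucent sort priority so it draws on top.
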(event `Defeat`
  (if (not (`self.isDefeated`))
    (set `self.isDefeated` true)
    (`PrimitiveComponent.SetCollisionEnabled` (`self.CapsuleComponent`) "NoCollision")
    (`MovementComponent.SetPlaneConstraintEnabled` (`self.CharacterMovement`) false)
    (`self.LaunchOnDefeat`)
    (`PaperZDAnimInstance.JumpToNode` (`self.GetAnimInstance`) "JumpDefeated" "None")
    (`PrimitiveComponent.SetTranslucentSortPriority` (`self.Sprite`) 1000)))

(fn `LaunchOnDefeat`
  (`self.LaunchCharacter` (+ (* (`KismetMathLibrary.Vector_Up`) (`self.DefeatedUpLaunch`)) (* (`KismetMathLibrary.Vector_Right`) (`self.DefeatedForwardLaunch`))) true true))

(fn `UserConstructionScript`)